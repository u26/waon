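; BP_KeyBoard is a musical keyboard actor that plays pitched notes with selectable equal-temperament or just-intonation tuning.
; BeginPlay builds both MIDI-indexed frequency tables from a base A4 pitch and creates a pool of MS_note audio components, one per key.
; Just intonation derives its root from the selected key's equal-tempered pitch, applying a repeating ratio table.
; KeyPressed looks up the active table and sets frequency and volume parameters before playing; KeyReleased stops that key's component.
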(event EventBeginPlay
  (CallFunction|SetKey "C")
  (CallFunction|SetOctave 3)
  (CallFunction|UpdateFrequency 4.4e+02)
  ;[1 0.7329 0.3846] make audio components
  (for _index (range 0 25)
    (bind _returnvalue (AddComponent|AddAudioComponent false))
    (Utilities|Array|Add (Variables|Default|Getaudio_components) _returnvalue)
    (Audio|Components|Audio|SetSound _returnvalue "/Game/Key/MS_note.MS_note")))

(event Collision|EventActorBeginOverlap
  (params (OtherActor :type Actor%20Object%20Reference)))

(event EventTick
  (params (DeltaSeconds :type Float%20%28single-precision%29)))

(fn ConstructionScript)

(fn UpdateEqualTemperation
  (params (base_pitch :type Float%20%28double-precision%29))
  (Utilities|Array|Clear (Variables|Default|Getfreq_equal))
  (Utilities|FlowControl|ForLoopwithBreak 0 128
    (:LoopBody
      (Utilities|Array|Add (Variables|Default|Getfreq_equal) 0.0))
    (:Completed
      (Utilities|Array|SetArrayElem (Variables|Default|Getfreq_equal) (LocalVariables|GetA4) base_pitch)
      (bind _index (Utilities|FlowControl|ForLoopwithBreak 70 127)
        (:LoopBody
          (LocalVariables|Settmp (* (Utilities|Array|Get(acopy) (Variables|Default|Getfreq_equal) (- _index 1)) 1.059463))
          (Utilities|Array|SetArrayElem (Variables|Default|Getfreq_equal) _index (LocalVariables|Gettmp)))
        (:Completed
          (LocalVariables|Setidx (LocalVariables|GetA4))
          (while (> (LocalVariables|Getidx) 0)
            (LocalVariables|Settmp (/ (Utilities|Array|Get(acopy) (Variables|Default|Getfreq_equal) (LocalVariables|Getidx)) 1.059463))
            (Math|Integer|DecrementInt (LocalVariables|Getidx)
              (:%20%20
                (Utilities|Array|SetArrayElem (Variables|Default|Getfreq_equal) (LocalVariables|Getidx) (LocalVariables|Gettmp))))))))))

(fn Play
  (params (Target :type Audio%20Parameter%20Controller%20Interface%20Interface) (freq :type Float%20%28single-precision%29%20%28by%20ref%29) (midi_idx :type Integer) (volume :type Float%20%28single-precision%29))
  (Development|PrintString (Utilities|String|ToString(Float) freq))
  (Audio|Parameter|SetFloatParameter Target "freq" freq :!class /Script/AudioExtensions.AudioParameterControllerInterface)
  (Audio|Parameter|SetFloatParameter Target "volume" volume :!class /Script/AudioExtensions.AudioParameterControllerInterface)
  (Audio|Components|Audio|Play (.AsAudio%20Component (Utilities|Casting|CastToAudioComponent Target)) 0.0))

(fn KeyPressed
  (params (key_index :type Integer))
  (bind _key_start_pos (Variables|Default|Getkey_start_pos))
  (bind _returnvalue (+ _key_start_pos key_index))
  (if (Utilities|Enum|Equal(Enum) (Variables|Default|Getmode) "NewEnumerator0")
    (LocalVariables|Setfreq (Utilities|Array|Get(acopy) (Variables|Default|Getfreq_equal) _returnvalue))
    (else
      (LocalVariables|Setfreq (Utilities|Array|Get(acopy) (Variables|Default|Getfreq_just) (+ (Variables|Default|Getkey_start_pos) key_index)))))
  (CallFunction|Play (Utilities|Array|Get(acopy) (Variables|Default|Getaudio_components) key_index) (LocalVariables|Getfreq) _returnvalue (Variables|Default|Getvolume))
  (Development|PrintString (Utilities|String|ToString(Integer) _returnvalue)))

(fn KeyReleased
  (params (key_idx :type Integer))
  (Audio|Components|Audio|Stop (Utilities|Array|Get(acopy) (Variables|Default|Getaudio_components) key_idx)))

(fn SetVolume
  (params (volume :type Float%20%28double-precision%29))
  (Variables|Default|Setvolume volume))

(fn UpdateJustInotation
  (bind _key_selected (Variables|Default|Getkey_selected))
  (bind _key (Variables|Default|Getkey))
  (bind _value (Utilities|Map|Find _key _key_selected))
  (bind _returnvalue (+ _value 12))
  (Utilities|Array|Clear (Variables|Default|Getfreq_just))
  (Utilities|FlowControl|ForLoopwithBreak 0 128
    (:LoopBody
      (Utilities|Array|Add (Variables|Default|Getfreq_just) 0.0))
    (:Completed
      ;[1 1 1] KEY0
      (LocalVariables|Setbase_pos _returnvalue)
      (LocalVariables|Setbase_freq (Utilities|Array|Get(acopy) (Variables|Default|Getfreq_equal) _returnvalue))
      (Utilities|Array|SetArrayElem (Variables|Default|Getfreq_just) (LocalVariables|Getbase_pos) (LocalVariables|Getbase_freq))
      (LocalVariables|Setidx (LocalVariables|Getbase_pos))
      (LocalVariables|Settmp_freq (LocalVariables|Getbase_freq))
      (while (< (LocalVariables|Getidx) 128) :!label _label
        (Utilities|Array|SetArrayElem (Variables|Default|Getfreq_just) (LocalVariables|Getidx) (* (LocalVariables|Gettmp_freq) (Utilities|Array|Get(acopy) (LocalVariables|Getjust_ratio) (LocalVariables|Getratio_idx))))
        (Development|PrintString (Utilities|String|ToString(Float) (Utilities|Array|Get(acopy) (Variables|Default|Getfreq_just) (LocalVariables|Getidx))))
        (Math|Integer|IncrementInt (LocalVariables|Getidx)
          (:%20%20
            (bind _result (Math|Integer|IncrementInt (LocalVariables|Getratio_idx))
              (:%20%20
                (if (> _result 11)
                  (LocalVariables|Setratio_idx 0)
                  (LocalVariables|Settmp_freq (* (LocalVariables|Gettmp_freq) 2.0))
                  (goto _label)
                  (else
                    (goto _label)))))))))))

(fn SetOctave
  (params (NewParam :type Integer))
  (Variables|Default|Setoctave (+ NewParam 1)))

(fn SetKey
  (params (key :type String))
  (Variables|Default|Setkey_selected key))

(fn UpdateFrequency
  (params (base_pitch :type Float%20%28double-precision%29))
  ;[0.6486 1 0.3636] Update frequency table
  (CallFunction|UpdateEqualTemperation base_pitch)
  (CallFunction|UpdateJustInotation))